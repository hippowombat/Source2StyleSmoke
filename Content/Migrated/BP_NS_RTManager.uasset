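; Manager actor that links a Niagara simulation to a ray-marched volume material on a static mesh through a shared 3D render target.
; The construction script creates a single-channel float volume target if none exists and passes it to Niagara.
; It briefly advances that component and a newly added one, then feeds the target and step limit to a dynamic material.
; The event graph does nothing; its delayed-activation GPU race workaround is disconnected.
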(event `self.ReceiveBeginPlay`)

(fn `UserConstructionScript`
  (bind _mi (`self.MI`))
  (bind _returnvalue (`AddComponent|NODE_AddNiagaraComponent-1`))
  (set `self.NS` _returnvalue)
  (if (not (`KismetSystemLibrary.IsValid` (`self.BPRT`)))
    (bind _returnvalue_2 (`KismetRenderingLibrary.CreateRenderTargetVolume` 128 128 128 "RTF_R32f"))
    (bind _output_get (set `self.BPRT` _returnvalue_2)))
  (bind _returnvalue_3 (`PrimitiveComponent.CreateDynamicMaterialInstance` (`self.StaticMesh`) 0 "/Game/Migrated/3DRayMarch_v3_param.3DRayMarch_v3_param" "test"))
  (set `self.MI` _returnvalue_3)
  (`NiagaraComponent.SetVariableTextureRenderTarget` (`self.Niagara`) "NTRT" _output_get)
  (`NiagaraComponent.AdvanceSimulation` (`self.Niagara`) 1 0.001)
  (`NiagaraComponent.AdvanceSimulation` (`self.NS`) 1 0.001)
  (`MaterialInstanceDynamic.SetTextureParameterValue` _mi "RT" (`self.BPRT`))
  (`MaterialInstanceDynamic.SetScalarParameterValue` _mi "maxSteps" (`KismetMathLibrary.Conv_IntToDouble` (`self.MaxSteps`))))