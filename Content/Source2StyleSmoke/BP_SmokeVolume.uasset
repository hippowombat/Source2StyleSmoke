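; Smoke volume actor that builds Source 2-style smoke flowing around obstacles, computed in the construction script.
; A breadth-first flood fill steps through six grid neighbors, using line traces to reject blocked cells, within a resolution-cubed cell budget.
; SmoothPointsToSphere trims points beyond a collision-adjusted average radius to round the shape.
; The points feed a Niagara array with cell-scaled sprites, with optional debug drawing.
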(event `self.ReceiveBeginPlay`)

(fn `BFS_FloodFill`
  (returns (ReturnPositions :type "Array of Vector Structure"))
  (locals (CheckedPositions :type "Array of Vector Structure") (PositionQueue :type "Array of Vector Structure") (AcceptedPositions :type "Array of Vector Structure") (FinalOutputPoints :type "Array of Vector Structure") (CurrentQueryPosition :type "Vector Structure") (TotalEnergy :type Integer) (TotalCollisions :type Integer) (CellSize :type "Float (double-precision)") (DidFindSpace :type Boolean))
  (bind _gridresolution (`self.GridResolution`))
  (bind _currentqueryposition (`local.CurrentQueryPosition`))
  (`KismetArrayLibrary.Array_Clear` (`local.CheckedPositions`))
  (`KismetArrayLibrary.Array_Clear` (`local.PositionQueue`))
  (`KismetArrayLibrary.Array_Clear` (`local.AcceptedPositions`))
  (set `local.TotalEnergy` (* _gridresolution _gridresolution _gridresolution))
  (set `local.CellSize` (/ (`self.TargetVolumeDiameter`) (`self.GridResolution`)))
  (`KismetArrayLibrary.Array_Add` (`local.PositionQueue`) (`self.K2_GetActorLocation`))
  (`KismetArrayLibrary.Array_Add` (`local.AcceptedPositions`) (`self.K2_GetActorLocation`))
  (`/Engine/EditorBlueprintResources/StandardMacros.DecrementInt` (`local.TotalEnergy`)
    (:`  `
      (`KismetArrayLibrary.Array_Add` (`local.CheckedPositions`) (`self.K2_GetActorLocation`))
      (while (and (> (`KismetArrayLibrary.Array_Length` (`local.PositionQueue`)) 0) (> (`local.TotalEnergy`) 0))
        (set `local.CurrentQueryPosition` (`KismetMathLibrary.SelectVector` (`KismetMathLibrary.Vector_SnappedToGrid` (`|GetArrayItem` (`local.PositionQueue`)) (`local.CellSize`)) (`|GetArrayItem` (`local.PositionQueue`)) (`self.SnapToGrid`)))
        (for _index (range 6)
          (bind _returnvalue (+ _currentqueryposition (* (`local.CellSize`) (select `int` _index :`0` (1.0 0.0 0.0) :`1` (-1.0 0.0 0.0) :`2` (0.0 1.0 0.0) :`3` (0.0 -1.0 0.0) :`4` (0.0 0.0 1.0) :`5` (0.0 0.0 -1.0) :!type "Vector Structure"))))
          (if (not (`KismetArrayLibrary.Array_Contains` (`local.CheckedPositions`) _returnvalue))
            (bind _outhit (`KismetSystemLibrary.LineTraceSingleForObjects` :`Start` _currentqueryposition :`End` _returnvalue :`ObjectTypes` (`|MakeArray` "ObjectTypeQuery1" "ObjectTypeQuery2" :!type "EObjectTypeQuery Enum") :`DrawTime` (`self.DebugDrawTime`)))
            (set `local.DidFindSpace` false)
            (bind (_bblockinghit _binitialoverlap _time _distance _location _impactpoint _normal _impactnormal _physmat _hitactor _hitcomponent _hitbonename _bonename _hititem _elementindex _faceindex _tracestart _traceend) (`GameplayStatics.BreakHitResult` _outhit))
            (if (not _bblockinghit)
              (`KismetArrayLibrary.Array_Add` (`local.PositionQueue`) _traceend)
              (`KismetArrayLibrary.Array_Add` (`local.AcceptedPositions`) _traceend)
              (set `local.DidFindSpace` true)
              (else
                (`/Engine/EditorBlueprintResources/StandardMacros.IncrementInt` (`local.TotalCollisions`)
                  (:`  `
                    _))))
            (`KismetArrayLibrary.Array_Add` (`local.CheckedPositions`) _traceend)
            (if (`local.DidFindSpace`)
              (`/Engine/EditorBlueprintResources/StandardMacros.DecrementInt` (`local.TotalEnergy`)))))
        (if (> (`KismetArrayLibrary.Array_Length` (`local.PositionQueue`)) 0)
          (`KismetArrayLibrary.Array_Remove` (`local.PositionQueue`))))
      (bind _outpoints (`self.SmoothPointsToSphere` (`local.AcceptedPositions`) (`local.TotalCollisions`)))
      (set `local.FinalOutputPoints` _outpoints)
      (if (> (`self.DebugDrawTime`) 0.0)
        (for _array_element (`local.FinalOutputPoints`)
          (`KismetSystemLibrary.DrawDebugBox` _array_element (`KismetMathLibrary.Conv_DoubleToVector` (* (`local.CellSize`) 0.5)) (struct :`G` 0.66 :`B` 0.66 :`A` 1.0) (`self.K2_GetActorRotation`) (`self.DebugDrawTime`) 2.5)
          (`KismetSystemLibrary.DrawDebugSphere` _array_element (* (`local.CellSize`) 0.1) 6 (struct :`R` 0.15 :`G` 0.5 :`B` 0.25 :`A` 1.0) (`self.DebugDrawTime`) 2.5)))
      (return (`local.FinalOutputPoints`)))))

(fn `SmoothPointsToSphere`
  (params (InPoints :type "Array of Vector Structure") (InAverageOffset :type Integer))
  (returns (OutPoints :type "Array of Vector Structure"))
  (locals (PointLengths :type "Array of Float (double-precision)") (LengthAverage :type "Float (double-precision)") (AveragedPoints :type "Array of Vector Structure"))
  (bind _lengthaverage (`local.LengthAverage`))
  (bind _returnvalue (- (`local.InAverageOffset`) (`KismetArrayLibrary.Array_Length` (`local.PointLengths`))))
  (for _array_element InPoints
    (`KismetArrayLibrary.Array_Add` (`local.PointLengths`) (`KismetMathLibrary.VSize` (`KismetMathLibrary.InverseTransformLocation` (`self.GetTransform`) _array_element))))
  (for _array_element_2 (`local.PointLengths`)
    (set `local.LengthAverage` (+ _array_element_2 (`local.LengthAverage`))))
  (set `local.LengthAverage` (+ (* _lengthaverage (`KismetMathLibrary.Clamp` _returnvalue 0 _returnvalue)) (/ _lengthaverage (`KismetMathLibrary.Conv_IntToDouble` (`KismetArrayLibrary.Array_Length` (`local.PointLengths`))))))
  (for _array_element_3 (`local.InPoints`)
    (bind _returnvalue_2 (`KismetMathLibrary.InverseTransformLocation` (`self.GetTransform`) _array_element_3))
    (bind _returnvalue_3 (`KismetMathLibrary.VSize` _returnvalue_2))
    (if (<= (`KismetMathLibrary.VSize` _returnvalue_2) (* (/ (`local.LengthAverage`) _returnvalue_3) _returnvalue_3))
      (`KismetArrayLibrary.Array_AddUnique` (`local.AveragedPoints`) (`KismetMathLibrary.TransformLocation` (`self.GetTransform`) (* (`KismetMathLibrary.Normal` _returnvalue_2) _returnvalue_3)))))
  (return (`local.AveragedPoints`)))

(fn `UserConstructionScript`
  (bind _ns_smokevolume (`self.NS_SmokeVolume`))
  (`KismetSystemLibrary.FlushPersistentDebugLines`)
  (`SphereComponent.SetSphereRadius` (`self.VolumeBounds`) (* (`self.TargetVolumeDiameter`) 0.5) true)
  (if (`self.FloodFillOnConstruct`)
    (bind _returnpositions (`self.BFS_FloodFill`))
    (set `self.VectorArray` _returnpositions)
    (`SceneComponent.SetVisibility` (`self.NS_SmokeVolume`) (`self.ShowParticles`) false)
    (if (`self.ShowParticles`)
      (`NiagaraComponent.ResetSystem` (`self.NS_SmokeVolume`))
      (`NiagaraDataInterfaceArrayFunctionLibrary.SetNiagaraArrayVector` _ns_smokevolume "VectorArray" (`self.VectorArray`))
      (`FXSystemComponent.SetFloatParameter` _ns_smokevolume "SpriteUniformScale" (* (/ (`self.TargetVolumeDiameter`) (`self.GridResolution`)) 2.0)))
    (else
      (`SceneComponent.SetVisibility` (`self.NS_SmokeVolume`) false false))))